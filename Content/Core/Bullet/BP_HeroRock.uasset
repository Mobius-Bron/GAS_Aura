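; BP_HeroRock is a hero projectile that reports ranged hits on enemies.
; Each tick it moves along its local Y axis by Speed, without scaling by delta time.
; When its Sphere overlaps a VirgoEnemyCharacter, it sends a Shared.Event.RangedHit gameplay event to its owner with that enemy as target, then destroys itself.
; It applies no damage in this graph, and other overlapped actors are ignored.
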(event `self.ReceiveTick`
  (params (DeltaSeconds :type "Float (single-precision)"))
  (`parent.ReceiveTick` DeltaSeconds)
  (`self.K2_AddActorLocalTransform` (`KismetMathLibrary.MakeTransform` (`KismetMathLibrary.MakeVector` 0.0 (`self.Speed`)))))

(event `self.Sphere.OnComponentBeginOverlap`
  (params (OverlappedComponent :type "PrimitiveComponent Object Reference") (OtherActor :type "Actor Object Reference") (OtherComp :type "PrimitiveComponent Object Reference") (OtherBodyIndex :type Integer) (bFromSweep :type Boolean) (SweepResult :type "HitResult Structure (by ref)"))
  (bind _asvirgo_enemy_character (cast `VirgoEnemyCharacter` OtherActor))
  (`AbilitySystemBlueprintLibrary.SendGameplayEventToActor` (`self.GetOwner`) (struct :`TagName` "Shared.Event.RangedHit") (make `GameplayEventData` (struct :`TagName` "Shared.Event.RangedHit") null _asvirgo_enemy_character))
  (`self.K2_DestroyActor`))

(fn `UserConstructionScript`
  (`parent.UserConstructionScript`))